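; Blueprint function library with two general utilities: a rotator-to-quaternion conversion and a query for actors that have meshes.
; RotatorToQuat builds the quaternion by hand from sines and cosines of the half roll, pitch and yaw angles.
; GetMeshActors scans every Actor in the world and returns those with at least one skeletal or static mesh component.
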(fn RotatortoQuat
  (params (Rotator :type Rotator))
  (bind (_roll _pitch _yaw) (Math|Rotator|BreakRotator Rotator))
  (bind _returnvalue (Math|Trig|DegreesToRadians _yaw))
  (bind _returnvalue_2 (Math|Trig|DegreesToRadians _roll))
  (bind _returnvalue_3 (Math|Trig|DegreesToRadians _pitch))
  (bind _returnvalue_4 (/ _returnvalue 2.0))
  (bind _returnvalue_5 (/ _returnvalue_2 2.0))
  (bind _returnvalue_6 (/ _returnvalue_3 2.0))
  (bind _returnvalue_7 (Math|Trig|Cos(Radians) _returnvalue_6))
  (bind _returnvalue_8 (Math|Trig|Sin(Radians) _returnvalue_6))
  (bind _returnvalue_9 (Math|Trig|Cos(Radians) _returnvalue_4))
  (bind _returnvalue_10 (Math|Trig|Sin(Radians) _returnvalue_4))
  (bind _returnvalue_11 (Math|Trig|Cos(Radians) _returnvalue_5))
  (bind _returnvalue_12 (Math|Trig|Sin(Radians) _returnvalue_5))
  (return (Class|KismetMathLibrary|MakeQuat (- (* _returnvalue_11 _returnvalue_8 _returnvalue_10) (* _returnvalue_12 _returnvalue_7 _returnvalue_9)) (- (* _returnvalue_11 _returnvalue_8 _returnvalue_9 -1.0) (* _returnvalue_12 _returnvalue_7 _returnvalue_10)) (- (* _returnvalue_11 _returnvalue_7 _returnvalue_10) (* _returnvalue_12 _returnvalue_8 _returnvalue_9)) (+ (* _returnvalue_11 _returnvalue_7 _returnvalue_9) (* _returnvalue_12 _returnvalue_8 _returnvalue_10)))))

(fn GetMeshActors
  (bind _outactors (Actor|GetAllActorsOfClass 0 "/Script/Engine.Actor"))
  (for _array_element _outactors
    (if (> (+ (Utilities|Array|Length (Actor|GetComponentsByClass _array_element "/Script/Engine.SkeletalMeshComponent")) (Utilities|Array|Length (Actor|GetComponentsByClass _array_element "/Script/Engine.StaticMeshComponent"))) 0)
      (Utilities|Array|Add (LocalVariables|GetMeshActors) _array_element)))
  (return (LocalVariables|GetMeshActors)))